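; Structural damage Blueprint that burns and collapses a section of house modules once every linked fire object is active.
; Tick counts active fires, then a timeline fades each module's ColorTint through dynamic material instances before swapping to a burnt material.
; After a delay, each module's root component tag selects a destructible mesh that replaces the static one and simulates physics.
; The fire objects are then hidden and fire and smoke particle templates are set.
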(event `self.ReceiveTick`
  (params (DeltaSeconds :type "Float (single-precision)"))
  (bind _fireobjects (`self.fireObjects`))
  (bind _housemodulesinvolved (`self.houseModulesInvolved`))
  (if (not (`self.sectionOnFire`))
    (for (_ _array_index) _fireobjects
      (set `self.activeFires` (+ (`self.activeFires`) (`/Game/Assets/Blueprints/FireSpreadBP.structFireActive` (`|GetArrayItem` _fireobjects _array_index)))))
    (if (== (`KismetArrayLibrary.Array_Length` _fireobjects) (`self.activeFires`))
      (set `self.sectionOnFire` true)
      (`KismetSystemLibrary.PrintString` "Section Completely On Fire")
      (for _array_element (`self.houseModulesInvolved`)
        (`self.BurnTransitionModule` _array_element))
      (bind (_direction _blend) (`Timeline|Línea de tiempo_0` :!via `PlayFromStart`)
        (:`Update`
          (for _array_element_2 _housemodulesinvolved
            (`MeshComponent.SetVectorParameterValueOnMaterials` (`StaticMeshActor.StaticMeshComponent` _array_element_2) "ColorTint" (`KismetMathLibrary.Conv_LinearColorToVector` (`KismetMathLibrary.LinearColorLerp` (`self.oldColor`) (`self.newColor`) _blend)))))
        (:`Finished`
          (set `self.oldColor` (`self.newColor`))
          (for _array_element_3 _housemodulesinvolved
            (bind _staticmeshcomponent (`StaticMeshActor.StaticMeshComponent` _array_element_3))
            (for (_ _array_index_2) (`MeshComponent.GetMaterials` _staticmeshcomponent)
              (`PrimitiveComponent.SetMaterial` _staticmeshcomponent _array_index_2 "/Game/Props/BurntMat/BurntMaterial1.BurntMaterial1")))
          (`KismetSystemLibrary.PrintString` "Wait 5 seconds for destruction")
          (`KismetSystemLibrary.Delay` 5.0)
          (`KismetSystemLibrary.PrintString` "Init destruction")
          (for _array_element_4 (`self.houseModulesInvolved`)
            (bind _staticmeshcomponent_2 (`StaticMeshActor.StaticMeshComponent` _array_element_4))
            (bind _returnvalue (`SceneComponent.GetRelativeTransform` _staticmeshcomponent_2))
            (bind _returnvalue_2 (`AddComponent|NODE_AddDestructibleComponent-0` :`self` _array_element_4 :`bManualAttachment` true :`RelativeTransform` _returnvalue))
            (`SceneComponent.K2_SetRelativeTransform` _returnvalue_2 _returnvalue false true)
            (bind _returnvalue_3 (`KismetStringLibrary.Conv_NameToString` (`|GetArrayItem` (`ActorComponent.ComponentTags` (`Actor.RootComponent` _array_element_4)))))
            (switch `string` _returnvalue_3
              (:`Default`
                (`KismetSystemLibrary.PrintString` _returnvalue_3))
              (:`Module05`
                (`DestructibleComponent.SetDestructibleMesh` _returnvalue_2 "/Game/HouseModules/0_5M/0_5_Metros_DM.0_5_Metros_DM")
                (`SceneComponent.SetVisibility` _staticmeshcomponent_2 false false :!label _label)
                (`self.SetActorEnableCollision` _array_element_4 false)
                (`PrimitiveComponent.SetSimulatePhysics` _returnvalue_2 true)
                (`KismetSystemLibrary.PrintString` "Destruction complete")
                (for _array_element_5 (`self.fireObjects`)
                  (`SceneComponent.SetVisibility` (`Actor.RootComponent` _array_element_5) false true)
                  (`ParticleSystemComponent.SetTemplate` (`self.FireVFX`) "/Game/StarterContent/Particles/P_Fire.P_Fire")
                  (`ParticleSystemComponent.SetTemplate` (`self.SmokeVFX`) "/Game/StarterContent/Particles/P_Smoke.P_Smoke")))
              (:`Module01`
                (`DestructibleComponent.SetDestructibleMesh` _returnvalue_2 "/Game/HouseModules/1M/1_Metro_DM.1_Metro_DM")
                (goto _label))
              (:`Module03`
                (`DestructibleComponent.SetDestructibleMesh` _returnvalue_2 "/Game/HouseModules/3M/3_Metros_DM.3_Metros_DM")
                (goto _label))
              (:`Corner01`
                (`DestructibleComponent.SetDestructibleMesh` _returnvalue_2 "/Game/HouseModules/Esquina1Metro/Esquina_1_Metro_DM.Esquina_1_Metro_DM")
                (goto _label))
              (:`Corner05`
                (`DestructibleComponent.SetDestructibleMesh` _returnvalue_2 "/Game/HouseModules/Esquina0_5Metros/Esquina_0_5_Metro_DM.Esquina_0_5_Metro_DM")
                (goto _label))
              (:`SmallWallWindow`
                (`DestructibleComponent.SetDestructibleMesh` _returnvalue_2 "/Game/HouseModules/ParedConVentanaPequeña/Pared_con_Ventana_Pequeña_DM.Pared_con_Ventana_Pequeña_DM")
                (goto _label))
              (:`BigWallWindow`
                (`DestructibleComponent.SetDestructibleMesh` _returnvalue_2 "/Game/HouseModules/ParedConVentanaGrande/Pared_con_Ventana_Grande_DM.Pared_con_Ventana_Grande_DM")
                (goto _label))
              (:`WallDoor`
                (`DestructibleComponent.SetDestructibleMesh` _returnvalue_2 "/Game/HouseModules/ParedConMarcoDePuerta/Pared_con_Marco_de_Puerta_DM.Pared_con_Marco_de_Puerta_DM")
                (goto _label))
              (:`Door`
                (`DestructibleComponent.SetDestructibleMesh` _returnvalue_2 "/Game/HouseModules/Door3/Door3_DM.Door3_DM")
                (goto _label))
              (:`Pilar`
                (`DestructibleComponent.SetDestructibleMesh` _returnvalue_2 "/Game/HouseModules/Pillar/Pilar_DM.Pilar_DM")
                (goto _label))
              (:`Roof`
                (`DestructibleComponent.SetDestructibleMesh` _returnvalue_2 "/Game/HouseModules/TechoGrande/TECHO_DM.TECHO_DM")
                (goto _label))))))
      (else
        (set `self.activeFires` 0)))))

(event `BurnTransitionModule`
  (params (ModuleMesh :type "StaticMeshActor Object Reference"))
  (bind _staticmeshcomponent (`StaticMeshActor.StaticMeshComponent` ModuleMesh))
  (bind _returnvalue (`PrimitiveComponent.CreateDynamicMaterialInstance` _staticmeshcomponent 0 (`PrimitiveComponent.GetMaterial` _staticmeshcomponent 0) "None"))
  (`PrimitiveComponent.SetMaterial` _staticmeshcomponent 0 _returnvalue)
  (bind _returnvalue_2 (`MaterialInstanceDynamic.K2_GetVectorParameterValue` _returnvalue "ColorTint"))
  (set `self.oldColor` _returnvalue_2)
  (set `self.newColor` (make `LinearColor` 0.0)))

(fn `UserConstructionScript`)