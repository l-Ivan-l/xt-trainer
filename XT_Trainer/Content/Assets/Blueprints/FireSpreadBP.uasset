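; FireSpreadBP is a burnable actor that catches fire and passes it on to nearby actors of the same class.
; FireSpread starts the fire particle effect and, in parallel, swaps the mesh material after a delay.
; After a shorter delay, it finds FireSpreadBP actors overlapping SpreadRadius with the Flammable tag and calls their FireSpread, creating a chain reaction.
; It removes its own Flammable tag before each such call.
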(event `FireSpread`
  (`|ExecutionSequence`
    (:`then_0`
      (`KismetSystemLibrary.Delay` 3.5)
      (`PrimitiveComponent.SetMaterial` (`self.Mesh`) 0 "/Game/VirtualReality/Materials/GenericHMDMaterial.GenericHMDMaterial"))
    (:`then_1`
      (`ParticleSystemComponent.SetTemplate` (`self.FireVFX`) "/Game/StarterContent/Particles/P_Fire.P_Fire")
      (`KismetSystemLibrary.Delay` 2.0)
      (for _array_element (`PrimitiveComponent.GetOverlappingActors` (`self.SpreadRadius`) "FireSpreadBP_C")
        (if (`self.ActorHasTag` _array_element "Flammable")
          (`KismetArrayLibrary.Array_RemoveItem` (`self.Tags`) "Flammable")
          (bind _asfire_spread_bp (cast `/Game/Assets/Blueprints/FireSpreadBP` _array_element))
          (`self.FireSpread` _asfire_spread_bp))))))

(fn `UserConstructionScript`)